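; BP_BaseCharacter is a base character using the Gameplay Ability System for melee combat, damage and death.
; It grants a melee ability on BeginPlay and activates it by indexed gameplay tag.
; DamageCapsule overlaps with characters of a different class apply a melee damage GameplayEffect at a random level and print the target's attribute for debugging.
; HP change events trigger a one-time death montage when HP reaches zero.
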(event `self.ReceiveBeginPlay`
  (`AbilitySystemComponent.K2_GiveAbility` (`self.AbilitySystem`) "/Game/Blueprints/Ability/00Melee/GAB_Melee.GAB_Melee_C" 0 -1)
  (add `self.HPChangeEvent` (delegate `HPChangeEvent_Event`)))

(event `HPChangeEvent_Event` :!signature `self.HPChangeEvent`
  (params (NewValue :type "Float (single-precision)"))
  (`self.IsDead` NewValue))

(event `Melee`
  (`self.Active Ability` 0))

(event `self.DamageCapsule.OnComponentBeginOverlap`
  (params (OverlappedComponent :type "PrimitiveComponent Object Reference") (OtherActor :type "Actor Object Reference") (OtherComp :type "PrimitiveComponent Object Reference") (OtherBodyIndex :type Integer) (bFromSweep :type Boolean) (SweepResult :type "HitResult Structure (by ref)"))
  (if (and (!= OtherActor self) (!= (`GameplayStatics.GetObjectClass` OtherActor) (`GameplayStatics.GetObjectClass` self)))
    (bind _asbp_base_character (cast `/Game/Blueprints/Character/BP_BaseCharacter` OtherActor))
    (`AbilitySystemComponent.BP_ApplyGameplayEffectToTarget` :`self` (`self.AbilitySystem`) :`GameplayEffectClass` "/Game/Blueprints/Ability/00Melee/GE_Melee_Damage.GE_Melee_Damage_C" :`Target` (`/Game/Blueprints/Character/BP_BaseCharacter.AbilitySystem` _asbp_base_character) :`Level` (`KismetMathLibrary.Conv_IntToDouble` (`KismetMathLibrary.RandomInteger` 3)))
    (`self.ShowHP` _asbp_base_character (struct :`AttributeName` "HP" :`Attribute` "/Script/GAS_Caroline.BaseAttributeSet:HP" :`AttributeOwner` "/Script/CoreUObject.Class'/Script/GAS_Caroline.BaseAttributeSet'"))))

(event `ShowHP`
  (params (Attribute :type "GameplayAttribute Structure"))
  (`KismetSystemLibrary.PrintString` (`KismetStringLibrary.Conv_DoubleToString` (`.ReturnValue` (`AbilitySystemBlueprintLibrary.GetFloatAttributeFromAbilitySystemComponent` (`self.AbilitySystem`) Attribute)))))

(event `IsDead`
  (params (HP :type "Float (double-precision)"))
  (if (and (<= HP 0.0) (not (`self.Dead`)))
    (set `self.Dead` true)
    (`|PlayMontage` (`self.Mesh`) "/Game/Animation/Montage/MA_Dead.MA_Dead")))

(fn `Active Ability`
  (params (AbilityIndex :type Integer))
  (`AbilitySystemComponent.TryActivateAbilitiesByTag` (`self.AbilitySystem`) (`|GetArrayItem` (`self.Gameplay Tag Container`) AbilityIndex) true))

(fn `UserConstructionScript`)