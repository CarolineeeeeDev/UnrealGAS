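; BP_Enemy is an AI-controlled enemy character that shows its health on an HP bar widget.
; It extends the parent's HP change event, setting the UMG_EnemyBar percent from the new value divided by an Ability System attribute.
; When that event finds the enemy dead, StopControl stops the brain component logic on its BP_AiPC controller.
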(event `self.HPChangeEvent_Event`
  (params (NewValue :type "Float (single-precision)"))
  (`parent.HPChangeEvent_Event` NewValue)
  (`/Game/Blueprints/Character/UMG/UMG_EnemyBar.SetPercent` (cast `/Game/Blueprints/Character/UMG/UMG_EnemyBar` (`WidgetComponent.GetUserWidgetObject` (`self.HPBar`)) :!pure true) (/ NewValue (`.ReturnValue` (`AbilitySystemBlueprintLibrary.GetFloatAttributeFromAbilitySystemComponent` (`self.AbilitySystem`) (struct :`AttributeName` "MaxHP" :`Attribute` "/Script/GAS_Caroline.BaseAttributeSet:MaxHP" :`AttributeOwner` "/Script/CoreUObject.Class'/Script/GAS_Caroline.BaseAttributeSet'")))))
  (if (`self.Dead`)
    (`self.StopControl`)))

(fn `StopControl`
  (bind _asbp_ai_pc (cast `/Game/Blueprints/Character/AI/00_Enemy/BP_AiPC` (`self.GetController`)))
  (`BrainComponent.StopLogic` (`AIController.BrainComponent` _asbp_ai_pc) "Dead"))

(fn `UserConstructionScript`
  (`parent.UserConstructionScript`))