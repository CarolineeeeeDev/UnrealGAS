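; Player character Blueprint that extends a parent character with GAS-based regeneration, HP bar updates and a camera lock mode.
; On BeginPlay it caches BP_PlayerController and grants and activates the BP_BaseRegen ability.
; HP change events update the controller's MainUI health bar and disable input once dead.
; LockCamera toggles between a raised, yaw-locked camera and free orbiting with movement-oriented rotation.
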(event `self.ReceiveBeginPlay`
  (`parent.ReceiveBeginPlay`)
  (bind _asbp_player_controller (cast `/Game/Blueprints/Gameplay/BP_PlayerController` (`GameplayStatics.GetPlayerController` 0)))
  (set `self.BP Player Controller` _asbp_player_controller)
  (`AbilitySystemComponent.K2_GiveAbilityAndActivateOnce` (`self.AbilitySystem`) "/Game/Blueprints/Ability/BaseRegen/BP_BaseRegen.BP_BaseRegen_C" 0 -1))

(event `self.HPChangeEvent_Event`
  (params (NewValue :type "Float (single-precision)"))
  (`parent.HPChangeEvent_Event` NewValue)
  (`/Game/Blueprints/Character/UMG/UMG_AttributeBar.SetPercent` (`/Game/Blueprints/Character/UMG/UMG_MainUI.UMG_AttributeBar_HP` (`/Game/Blueprints/Gameplay/BP_PlayerController.MainUI` (`self.BP Player Controller`))) (/ NewValue (`.ReturnValue` (`AbilitySystemBlueprintLibrary.GetFloatAttributeFromAbilitySystemComponent` (`self.AbilitySystem`) (struct :`AttributeName` "MaxHP" :`Attribute` "/Script/GAS_Caroline.BaseAttributeSet:MaxHP" :`AttributeOwner` "/Script/CoreUObject.Class'/Script/GAS_Caroline.BaseAttributeSet'")))))
  (if (`self.Dead`)
    (`self.DisableInput` (`self.BP Player Controller`) null)))

(fn `LockCamera`
  (params (Lock :type Boolean))
  (bind _camera (`self.Camera`))
  (if Lock
    (set `SpringArmComponent.bUsePawnControlRotation` false (`self.SpringArm`))
    (set `CharacterMovementComponent.bOrientRotationToMovement` false (`self.CharacterMovement`))
    (set `self.bUseControllerRotationYaw` true)
    (`SceneComponent.K2_SetRelativeLocationAndRotation` _camera (0.0 0.0 200.0) (struct :`Pitch` -20.0) true false)
    (else
      (set `SpringArmComponent.bUsePawnControlRotation` true (`self.SpringArm`))
      (set `CharacterMovementComponent.bOrientRotationToMovement` true (`self.CharacterMovement`))
      (set `self.bUseControllerRotationYaw` false)
      (`SceneComponent.K2_SetRelativeLocationAndRotation` :`self` _camera :`bSweep` true))))

(fn `UserConstructionScript`
  (`parent.UserConstructionScript`))