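; BPF_Lib is a small Blueprint function library of player lookup and direction helpers.
; GetPlayerAndPC casts the index 0 character and controller to BP_Player and BP_PlayerController and returns both, stopping if either cast fails.
; GetPlayerToActorDir builds on it to return the normalized direction from the player to a target actor, or a zero vector when the target is invalid.
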(fn `GetPlayerAndPC`
  (returns (`BP Player` :type "/Game/Blueprints/Character/BP_Player Object Reference") (`BP Controller` :type "/Game/Blueprints/Gameplay/BP_PlayerController Object Reference"))
  (bind _asbp_player (cast `/Game/Blueprints/Character/BP_Player` (`GameplayStatics.GetPlayerCharacter` (`local.__WorldContext`))))
  (bind _asbp_player_controller (cast `/Game/Blueprints/Gameplay/BP_PlayerController` (`GameplayStatics.GetPlayerController` null)))
  (return _asbp_player _asbp_player_controller))

(fn `GetPlayerToActorDir`
  (params (Target :type "Actor Object Reference"))
  (returns (Dir :type "Vector Structure"))
  (`/Engine/EditorBlueprintResources/StandardMacros.IsValid` Target
    (:`Is Valid`
      (return (`KismetMathLibrary.Normal` (- (`Actor.K2_GetActorLocation` Target) (`Actor.K2_GetActorLocation` (`self.GetPlayerAndPC` (`local.__WorldContext`)))))))
    (:`Is Not Valid`
      (return (0.0 0.0 0.0)))))